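; Wizard character Blueprint with a stagger-driven active ragdoll, a HUD, and a game-over exit.
; BeginPlay adds the HUD and applies physical animation below the pelvis for active ragdoll.
; Any damage, including self-damage from Space or 1, drains Stagger; Tick switches to full ragdoll once it empties.
; Tick also checks Lives, showing Game Over at zero, then destroying the actor and quitting after a delay.
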(event `self.ReceiveTick`
  (params (DeltaSeconds :type "Float (single-precision)"))
  (`|ExecutionSequence`
    (:`then_0`
      (if (<= (`self.lives`) 0)
        (bind _returnvalue (`|CreateWidget` "/Game/UI/Game_Over.Game_Over_C"))
        (`UserWidget.AddToViewport` _returnvalue 0)
        (`KismetSystemLibrary.Delay` 3.0)
        (`self.K2_DestroyActor`)
        (`KismetSystemLibrary.QuitGame` null "Quit")))
    (:`then_1`
      (`self.staggerSystem`))))

(event `self.ReceiveBeginPlay`
  (`|ExecutionSequence`
    (:`then_0`
      (`self.active ragdoll`))
    (:`then_1`
      (bind _returnvalue (`|CreateWidget` "/Game/UI/game_HUD.game_HUD_C"))
      (`UserWidget.AddToViewport` _returnvalue 0))))

(event `Key|SpaceBar`
  (params (Key :type "Key Structure"))
  (:`Pressed`
    (`GameplayStatics.ApplyDamage` self 10.0 :!label _label)))

(event `Key|One`
  (params (Key :type "Key Structure"))
  (:`Pressed`
    (goto _label)))

(event `self.ReceiveAnyDamage`
  (params (Damage :type "Float (single-precision)") (DamageType :type "DamageType Object Reference") (InstigatedBy :type "Controller Object Reference") (DamageCauser :type "Actor Object Reference"))
  (set `self.stagger` (- (`self.stagger`) Damage)))

(fn `active ragdoll`
  (`PhysicalAnimationComponent.SetSkeletalMeshComponent` (`self.PhysicalAnimation`) (`self.Mesh`))
  (`PhysicalAnimationComponent.ApplyPhysicalAnimationSettingsBelow` (`self.PhysicalAnimation`) "pelvis" (make `PhysicalAnimationData` true 1000.0 100.0 1000.0 100.0 100.0 100.0) true)
  (`SkeletalMeshComponent.SetAllBodiesBelowSimulatePhysics` (`self.Mesh`) "pelvis" true false))

(fn `disable active ragdoll`
  (`PhysicalAnimationComponent.SetSkeletalMeshComponent` (`self.PhysicalAnimation`) (`self.Mesh`))
  (`PhysicalAnimationComponent.ApplyPhysicalAnimationSettingsBelow` (`self.PhysicalAnimation`) "pelvis" (make `PhysicalAnimationData` true) true)
  (`SkeletalMeshComponent.SetAllBodiesBelowSimulatePhysics` (`self.Mesh`) "pelvis" true false))

(fn `ragdoll`
  (bind _mesh (`self.Mesh`))
  (`|ExecutionSequence`
    (:`then_0`
      (`CharacterMovementComponent.SetMovementMode` (`self.CharacterMovement`) "MOVE_None" 0))
    (:`then_1`
      (`PrimitiveComponent.SetCollisionEnabled` (`self.CapsuleComponent`) "NoCollision")
      (`PrimitiveComponent.SetCollisionObjectType` _mesh "ECC_PhysicsBody")
      (`PrimitiveComponent.SetCollisionEnabled` _mesh "QueryAndPhysics")
      (`SkeletalMeshComponent.SetAllBodiesBelowSimulatePhysics` _mesh "pelvis" true true))
    (:`then_2`
      (`self.StopAnimMontage` null))))

(fn `staggerSystem`
  (if (<= (`self.stagger`) 0.0)
    (`self.disable active ragdoll`)
    (`self.ragdoll`)))

(fn `UserConstructionScript`)