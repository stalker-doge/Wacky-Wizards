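; Jump pad actor that launches any Character overlapping its trigger component along the forward vector of its Arrow.
; The overlap makes the character jump, waits briefly, then calls LaunchCharacter without overriding existing velocity.
; A DoOnce blocks retriggering until the launch finishes.
; A timeline meant to tilt the pad's pitch is present but never runs.
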(event `self.rrr.OnComponentBeginOverlap`
  (params (OverlappedComponent :type "PrimitiveComponent Object Reference") (OtherActor :type "Actor Object Reference") (OtherComp :type "PrimitiveComponent Object Reference") (OtherBodyIndex :type Integer) (bFromSweep :type Boolean) (SweepResult :type "HitResult Structure (by ref)"))
  (bind _ascharacter (cast `Character` OtherActor))
  (`/Engine/EditorBlueprintResources/StandardMacros.DoOnce` false :!label _label
    (:`Completed`
      (`Character.Jump` _ascharacter)
      (`KismetSystemLibrary.Delay` 0.2)
      (`Character.LaunchCharacter` _ascharacter (* (`SceneComponent.GetForwardVector` (`self.Arrow`)) 2000.0) false false)
      (goto _label :!via `Reset`))))

(fn `UserConstructionScript`)