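; Game mode for Wacky Wizards that sets up local multiplayer with one wizard per PlayerStart in the level.
; On BeginPlay it loops over the PlayerStarts, creating local players, adding an Enhanced Input mapping context, then spawning and possessing a WizardBP at each start, with player 0 using the existing controller.
; Helper functions order spawns by numeric PlayerStartTag, but BeginPlay never calls them, so player-to-start assignment follows actor query order.
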(event `self.ReceiveBeginPlay`
  (bind _returnvalue (`GameplayStatics.GetPlayerController` 0))
  (bind _outactors (`GameplayStatics.GetAllActorsOfClass` "/Script/Engine.PlayerStart"))
  (for (_array_element _array_index) _outactors
    (bind _output_get (set `self.Array Index` _array_index))
    (bind _returnvalue_2 (`GameplayStatics.CreatePlayer` _output_get))
    (if (> (`self.Array Index`) 0)
      (`EnhancedInputSubsystemInterface.AddMappingContext` (pcsubsystem `EnhancedInputLocalPlayerSubsystem` _returnvalue_2) null 0 (struct))
      (bind _returnvalue_3 (`self.GetTransform` _array_element))
      (bind _returnvalue_4 (`|SpawnActorFromClass` "/Game/WW_STUFF/GameDesign/GameDesign_Blueprints/WizardBP.WizardBP_C" _returnvalue_3 "Undefined" "MultiplyWithRoot" null null))
      (`Controller.Possess` (`GameplayStatics.GetPlayerController` (`self.Array Index`)) _returnvalue_4)
      (else
        (`EnhancedInputSubsystemInterface.AddMappingContext` (pcsubsystem `EnhancedInputLocalPlayerSubsystem` _returnvalue) null 0 (struct))
        (bind _returnvalue_5 (`|SpawnActorFromClass` "/Game/WW_STUFF/GameDesign/GameDesign_Blueprints/WizardBP.WizardBP_C" _returnvalue_3 "Undefined" "MultiplyWithRoot" null null))
        (`Controller.Possess` _returnvalue _returnvalue_5)))))

(fn `Get Player Start Points`
  (bind _outactors (`GameplayStatics.GetAllActorsOfClass` "/Script/Engine.PlayerStart"))
  (set `self.Player Start Array` _outactors))

(fn `Name to int`
  (params (`Player Start` :type "PlayerStart Object Reference"))
  (returns (ReturnValue :type Integer))
  (return (`KismetStringLibrary.Conv_StringToInt` (`KismetStringLibrary.Conv_NameToString` (`PlayerStart.PlayerStartTag` `Player Start`)))))

(fn `Spawn Input Receivers`
  (locals (Index :type Integer))
  (bind _player_start_array (`self.Player Start Array`))
  (bind _index (`local.Index`))
  (for (_ _array_index) _player_start_array
    (set `local.Index` _array_index)
    (for _array_element _player_start_array
      (if (== (`self.Name to int` _array_element) (`local.Index`))
        (`GameplayStatics.CreatePlayer` _index)
        (`|SpawnActorFromClass` "/Game/WW_STUFF/GameDesign/GameDesign_Blueprints/WizardBP.WizardBP_C" (`self.GetTransform` (`|GetArrayItem` (`self.Player Start Array`) _index)) "Undefined" "MultiplyWithRoot" null null)))))

(fn `UserConstructionScript`)